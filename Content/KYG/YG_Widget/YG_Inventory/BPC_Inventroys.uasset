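; Inventory component that stores item class and amount pairs in a slot array, sized at BeginPlay from the player's WeaponInventorySlots.
; AddItem writes to the first empty slot and returns whether one was found; it reads MaxStackAmount but does no stacking.
; Each successful add refreshes the matching widget slot in the inventory grid on the player's Overlay.
; GetItemDataAtIndex exposes a slot's item and amount.
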(event EventBeginPlay
  (Utilities|Array|Resize (Variables|Default|GetInventory%20Slots) (Variables|/Script/OneSoul.OnsSoulPlayer|GetWeaponInventorySlots (.AsBP%20Player (Utilities|Casting|CastToBP_Player (Game|GetPlayerCharacter 0))))))

(fn AddItem
  (params (Item :type BP%20Inventroy%20Master%20Class%20Reference) (Amount :type Integer))
  (bind (_success_ _index) (CallFunction|CheckforEmptySlot))
  (LocalVariables|SetLocal%20Item Item)
  (LocalVariables|SetLocal%20Amount Amount)
  (LocalVariables|SetLocal%20Max%20Stack%20Amount (.MaxStackAmount (Utilities|Struct|BreakS_ItemData (Utilities|GetClassDefaults (LocalVariables|GetLocal%20Item)))))
  (if _success_
    (LocalVariables|SetLocal%20Index _index)
    (Utilities|Array|SetArrayElem (Variables|Default|GetInventory%20Slots) (LocalVariables|GetLocal%20Index) (Utilities|Struct|MakeS_InventoryItems (LocalVariables|GetLocal%20Item) (LocalVariables|GetLocal%20Amount)))
    (CallFunction|UpdataInventorySlot (LocalVariables|GetLocal%20Index))
    (return true)
    (else
      (return false))))

(fn CheckforEmptySlot
  (bind (_array_element _array_index) (Utilities|Array|ForEachLoopwithBreak (Variables|Default|GetInventory%20Slots) :!label _label)
    (:LoopBody
      (if (Utilities|IsValidClass (.Item (Utilities|Struct|BreakS_InventoryItems _array_element)))
        (LocalVariables|SetLocal%20Success false)
        (else
          (LocalVariables|SetLocal%20Success true)
          (LocalVariables|SetLocal%20Index _array_index)
          (goto _label Break))))
    (:Completed
      (return (LocalVariables|GetLocal%20Success) (LocalVariables|GetLocal%20Index)))))

(fn GetItemDataatIndex
  (params (Index :type Integer))
  (bind _inventory_slots (Variables|Default|GetInventory%20Slots))
  (bind _output (Utilities|Array|Get(acopy) _inventory_slots Index))
  (bind (_item _amount) (Utilities|Struct|BreakS_InventoryItems _output))
  (return _item _amount))

(fn UpdataInventorySlot
  (params (Index :type Integer))
  (Default|UpdateSlot (Utilities|Array|Get(acopy) (Variables|/Game/KYG/YG_Widget/YG_Inventory/W_InventoryGrid.W_InventoryGrid_C|GetSlotArray (Variables|/Game/KYG/YG_Widget/WBP_OneSoulOverlay.WBP_OneSoulOverlay_C|GetW_InventoryGrid (Variables|/Game/KYG/YG_Character/BP_Player.BP_Player_C|GetOverlay (.AsBP%20Player (Utilities|Casting|CastToBP_Player (Game|GetPlayerCharacter 0)))))) Index)))