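; Master weapon pickup actor that adds its item and amount to the player's inventory component.
; Sphere overlap stores the player, calls the pickup and starts per-tick checks; end overlap stops them.
; Tick enables actor input only while a visibility trace to the player is unblocked and within pickup distance.
; A successful add keeps any remainder as the new amount, otherwise destroys the actor.
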(event OnComponentBeginOverlap(Sphere)
  (params (OverlappedComponent :type Primitive%20Component%20Object%20Reference) (OtherActor :type Actor%20Object%20Reference) (OtherComp :type Primitive%20Component%20Object%20Reference) (OtherBodyIndex :type Integer) (bFromSweep :type Boolean) (SweepResult :type Hit%20Result%20Structure%20%28by%20ref%29))
  (bind _asbp_player (Utilities|Casting|CastToBP_Player OtherActor))
  (Variables|Default|SetPlayer _asbp_player)
  (Variables|Default|SetUpdateActor true)
  (CallFunction|PickupWeapon))

(event OnComponentEndOverlap(Sphere)
  (params (OverlappedComponent :type Primitive%20Component%20Object%20Reference) (OtherActor :type Actor%20Object%20Reference) (OtherComp :type Primitive%20Component%20Object%20Reference) (OtherBodyIndex :type Integer))
  (Utilities|Casting|CastToBP_Player OtherActor)
  (Variables|Default|SetUpdateActor false)
  (Input|DisableInput (Game|GetPlayerController 0)))

(event Custom|Pickup_Weapon
  (bind (_success_ _remainder) (Default|AddWeapon (Variables|/Game/KYG/YG_Character/BP_Player.BP_Player_C|GetBPC_Inventory (Variables|Default|GetPlayer)) (Variables|Default|GetItem) (Variables|Default|GetAmount)))
  (if _success_
    (if (> _remainder 0)
      (Variables|Default|SetAmount _remainder)
      (else
        (Actor|DestroyActor)))))

(event EventTick
  (params (DeltaSeconds :type Float%20%28single-precision%29))
  (bind _returnvalue (Game|GetPlayerController 0))
  (if (Variables|Default|GetUpdateActor)
    (bind (_outhit _returnvalue_2) (Collision|LineTraceByChannel (Transformation|GetActorLocation) (Transformation|GetActorLocation (Variables|Default|GetPlayer)) "TraceTypeQuery1" false 0 "None"))
    (if (not _returnvalue_2)
      (if (<= (Math|Vector|VectorLength (- (.TraceStart (Collision|BreakHitResult _outhit)) (.TraceEnd (Collision|BreakHitResult _outhit)))) (Variables|Default|GetPickUpDistance))
        (Input|EnableInput _returnvalue)
        (else
          (Input|DisableInput _returnvalue)))
      (else
        (Input|DisableInput (Game|GetPlayerController 0))))))

(fn ConstructionScript)