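; Actor component that holds equipped items in separate weapon and shield ("Sheid") slot arrays.
; BeginPlay sizes both arrays from slot counts on BP_Player.
; Add functions write item and amount into the first empty slot, return success, then call slot update functions, which are empty stubs.
; Getters return item and amount by index; max stack amount is read but never enforced.
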(event EventBeginPlay
  (bind _returnvalue (Game|GetPlayerCharacter 0))
  (bind _asbp_player (Utilities|Casting|CastToBP_Player _returnvalue))
  (Utilities|Array|Resize (Variables|Default|GetWeapon%20Slots) (Variables|/Script/OneSoul.OnsSoulPlayer|GetWeaponEquipmentSlots _asbp_player))
  (Utilities|Array|Resize (Variables|Default|GetSheid%20Slots) (Variables|/Script/OneSoul.OnsSoulPlayer|GetSheidEquipmentSlots _asbp_player)))

(fn AddWeapon
  (params (Item :type BP%20Weapon%20Inventory%20Item%20Mater%20Class%20Reference) (Amount :type Integer) (itemdata :type S%20Weapon%20Data%20Structure))
  (bind (_success_ _index) (CallFunction|CheckOfWeaponEmptySlot))
  (LocalVariables|SetLocalWeaponData itemdata)
  (LocalVariables|SetLocal%20Weapon Item)
  (LocalVariables|SetLocal%20Amount Amount)
  (LocalVariables|SetLocalMax%20Stack%20Amount (.MaxStackAmount (Utilities|Struct|BreakS_WeaponData (Utilities|GetClassDefaults (LocalVariables|GetLocal%20Weapon)))))
  (if _success_
    (LocalVariables|SetLocal%20Index _index)
    (Utilities|Array|SetArrayElem (Variables|Default|GetWeapon%20Slots) (LocalVariables|GetLocal%20Index) (Utilities|Struct|MakeS_WeaponItems (LocalVariables|GetLocal%20Weapon) (LocalVariables|GetLocal%20Amount)))
    (CallFunction|UpdateWeaponSlot self (LocalVariables|GetLocal%20Index) (LocalVariables|GetLocalWeaponData))
    (return true)
    (else
      (return false))))

(fn AddSheid
  (params (Item :type BP%20Sheid%20Inventory%20Item%20Mater%20Class%20Reference) (Amount :type Integer))
  (bind (_success_ _index) (CallFunction|CheckOfSheidEmptySlot))
  (LocalVariables|SetLocal%20Sheid Item)
  (LocalVariables|SetLocal%20Amount Amount)
  (LocalVariables|SetLocal%20Max%20Stack%20Amount (.MaxStackAmount (Utilities|Struct|BreakS_SheidData (Utilities|GetClassDefaults (LocalVariables|GetLocal%20Sheid)))))
  (if _success_
    (LocalVariables|SetLocal%20Index _index)
    (Utilities|Array|SetArrayElem (Variables|Default|GetSheid%20Slots) (LocalVariables|GetLocal%20Index) (Utilities|Struct|MakeS_SheidItems (LocalVariables|GetLocal%20Sheid) (LocalVariables|GetLocal%20Amount)))
    (CallFunction|UpdateSheidSlot (LocalVariables|GetLocal%20Index))
    (return true)
    (else
      (return false))))

(fn CheckOfWeaponEmptySlot
  (bind (_array_element _array_index) (Utilities|Array|ForEachLoopwithBreak (Variables|Default|GetWeapon%20Slots) :!label _label)
    (:LoopBody
      (if (Utilities|IsValidClass (.Item (Utilities|Struct|BreakS_WeaponItems _array_element)))
        (LocalVariables|SetLocalSuccess false)
        (else
          (LocalVariables|SetLocalSuccess true)
          (LocalVariables|SetLocalIndex _array_index)
          (goto _label Break))))
    (:Completed
      (return (LocalVariables|GetLocalSuccess) (LocalVariables|GetLocalIndex)))))

(fn CheckOfSheidEmptySlot
  (bind (_array_element _array_index) (Utilities|Array|ForEachLoopwithBreak (Variables|Default|GetSheid%20Slots) :!label _label)
    (:LoopBody
      (if (Utilities|IsValidClass (.Item (Utilities|Struct|BreakS_SheidItems _array_element)))
        (LocalVariables|SetLocalSuccess false)
        (else
          (LocalVariables|SetLocalSuccess true)
          (LocalVariables|SetLocalIndex _array_index)
          (goto _label Break))))
    (:Completed
      (return (LocalVariables|GetLocalSuccess) (LocalVariables|GetLocalIndex)))))

(fn GetWeaponDataatIndex
  (params (Index :type Integer))
  (bind _weapon_slots (Variables|Default|GetWeapon%20Slots))
  (bind _output (Utilities|Array|Get(acopy) _weapon_slots Index))
  (bind (_item _amount) (Utilities|Struct|BreakS_WeaponItems _output))
  (return _item _amount))

(fn GetSheidDataatIndex
  (params (Index :type Integer))
  (bind _sheid_slots (Variables|Default|GetSheid%20Slots))
  (bind _output (Utilities|Array|Get(acopy) _sheid_slots Index))
  (bind (_item _amount) (Utilities|Struct|BreakS_SheidItems _output))
  (return _item _amount))

(fn UpdateWeaponSlot
  (params (Index :type Integer) (weapondata :type S%20Weapon%20Data%20Structure)))

(fn UpdateSheidSlot
  (params (Index :type Integer)))