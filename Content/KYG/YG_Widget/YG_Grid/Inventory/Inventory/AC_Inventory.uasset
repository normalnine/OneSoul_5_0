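; Inventory component that sets up fixed-size item storage for the grid inventory UI.
; It holds four category arrays for weapons, shields, upgrades and user items.
; InitializeInventory forwards to a CL_InitializeInventory event, which resizes each array to the AmountofSlots value.
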(event Custom|InitializeInventory
  (CallFunction|CLInitializeInventory))

(event Custom|CL_InitializeInventory
  (bind _amountofslots (Variables|Default|GetAmountofSlots))
  (Utilities|Array|Resize (Variables|Default|GetWeaponCategory) _amountofslots)
  (Utilities|Array|Resize (Variables|Default|GetSheidCategory) _amountofslots)
  (Utilities|Array|Resize (Variables|Default|GetUpgradeCategory) _amountofslots)
  (Utilities|Array|Resize (Variables|Default|GetUserItemCategory) _amountofslots))