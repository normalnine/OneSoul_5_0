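; BP_Home_and_Start is a trigger actor that sends the player either to another level or to another spot in the current map.
; When BP_Player overlaps its box, it fades the camera to dark blue and plays a teleport sound.
; The yaw of the player's world location vector picks the branch.
; After a short delay, it either opens First-Person_Demo_V2 or moves the player to a fixed position and fades back in.
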(event OnComponentBeginOverlap(Box)
  (params (OverlappedComponent :type Primitive%20Component%20Object%20Reference) (OtherActor :type Actor%20Object%20Reference) (OtherComp :type Primitive%20Component%20Object%20Reference) (OtherBodyIndex :type Integer) (bFromSweep :type Boolean) (SweepResult :type Hit%20Result%20Structure%20%28by%20ref%29))
  (bind _asbp_player (Utilities|Casting|CastToBP_Player OtherActor))
  (CameraFades|StartCameraFade (Game|GetPlayerCameraManager 0) 0.0 1.0 2.0 "(R=0.000000,G=0.004511,B=0.098958,A=1.000000)" false false)
  (Audio|PlaySound2D "/Game/LJW/Enemys/sound/88_Teleport_02.88_Teleport_02" 1.0 1.0 0.0 0 0)
  (if (> (.Yaw (Math|Vector|GetYawPitchfromVector (Transformation|GetActorLocation _asbp_player))) -2e+01)
    (Utilities|FlowControl|Delay 1.5)
    (Game|OpenLevel(byName) "First-Person_Demo_V2")
    (else
      (Utilities|FlowControl|Delay 1.5)
      (Transformation|SetActorLocationAndRotation _asbp_player "-1500.000000,-7006.349121,700.400391")
      (CameraFades|StartCameraFade (Game|GetPlayerCameraManager 0) 1.0 0.0 1.5 "(R=0.000000,G=0.004511,B=0.098958,A=1.000000)" false false))))

(event EventBeginPlay)

(event Collision|EventActorBeginOverlap
  (params (OtherActor :type Actor%20Object%20Reference)))

(event EventTick
  (params (DeltaSeconds :type Float%20%28single-precision%29)))

(fn ConstructionScript)