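; BP_TP_Random is a random teleport trigger for BP_Player, fired when the player overlaps its Box.
; It fades the camera to dark navy, plays a teleport sound and, after a short delay, picks one of four hardcoded locations.
; Only the first branch moves the player and prints a debug random number; the other three only set RanLoc, and no fade-in follows.
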(event OnComponentBeginOverlap(Box)
  (params (OverlappedComponent :type Primitive%20Component%20Object%20Reference) (OtherActor :type Actor%20Object%20Reference) (OtherComp :type Primitive%20Component%20Object%20Reference) (OtherBodyIndex :type Integer) (bFromSweep :type Boolean) (SweepResult :type Hit%20Result%20Structure%20%28by%20ref%29))
  (bind _returnvalue (Math|Random|RandomIntegerinRange 0 3))
  (bind _asbp_player (Utilities|Casting|CastToBP_Player OtherActor))
  (CameraFades|StartCameraFade (Game|GetPlayerCameraManager 0) 0.0 1.0 2.0 "(R=0.000000,G=0.004511,B=0.098958,A=1.000000)" false false)
  (Audio|PlaySound2D "/Game/LJW/Enemys/sound/88_Teleport_02.88_Teleport_02" 1.0 1.0 0.0 0 0)
  (Utilities|FlowControl|Delay 1.5)
  (switch int _returnvalue
    (:0
      (Variables|Default|SetRanLoc "600.000000,894.000000,-1352.000000")
      (Transformation|SetActorLocationAndRotation _asbp_player (Variables|Default|GetRanLoc))
      (Development|PrintString (Utilities|String|ToString(Integer) _returnvalue)))
    (:1
      (Variables|Default|SetRanLoc "1784.000000,292.000000,-2961.000000"))
    (:2
      (Variables|Default|SetRanLoc "546.000000,894.000000,-1352.000000"))
    (:3
      (Variables|Default|SetRanLoc "546.000000,894.000000,-1352.000000"))))

(event EventBeginPlay)

(event Collision|EventActorBeginOverlap
  (params (OtherActor :type Actor%20Object%20Reference)))

(event EventTick
  (params (DeltaSeconds :type Float%20%28single-precision%29)))

(fn ConstructionScript)