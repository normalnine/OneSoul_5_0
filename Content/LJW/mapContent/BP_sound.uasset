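; BP_sound is a map music controller that switches 2D tracks around a boss encounter.
; BeginPlay starts an ambient Skyrim track and keeps its audio component in NewVar0.
; When BP_Player enters the Box trigger, it swaps to a Dark Souls III boss theme and destroys the Box so it fires once.
; Tick polls the player's Killtitan flag and, via DoOnce, restores the ambient track.
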(event OnComponentBeginOverlap(Box)
  (params (OverlappedComponent :type Primitive%20Component%20Object%20Reference) (OtherActor :type Actor%20Object%20Reference) (OtherComp :type Primitive%20Component%20Object%20Reference) (OtherBodyIndex :type Integer) (bFromSweep :type Boolean) (SweepResult :type Hit%20Result%20Structure%20%28by%20ref%29))
  (Utilities|Casting|CastToBP_Player OtherActor)
  (Audio|Components|Audio|Stop (Variables|Default|GetNewVar_0))
  (bind _returnvalue (Audio|SpawnSound2D "/Game/LJW/mapContent/BackgroundMusic/DarkSoulsIII__Vordt_Theme_of_the_Boreal_Valley.DarkSoulsIII__Vordt_Theme_of_the_Boreal_Valley" 1.0 1.0 0.0 0))
  (Variables|Default|SetNewVar_0 _returnvalue)
  (Components|DestroyComponent (Variables|Default|GetBox)))

(event EventBeginPlay
  (bind _returnvalue (Audio|SpawnSound2D "/Game/LJW/mapContent/BackgroundMusic/Skyrim_Soundtrack__Silence_Unbroken.Skyrim_Soundtrack__Silence_Unbroken" 1.0 1.0 0.0 0 false false))
  (Variables|Default|SetNewVar_0 _returnvalue))

(event Collision|EventActorBeginOverlap
  (params (OtherActor :type Actor%20Object%20Reference)))

(event EventTick
  (params (DeltaSeconds :type Float%20%28single-precision%29))
  (bind _asbp_player (Utilities|Casting|CastToBP_Player (Game|Player|GetPlayerPawn 0)))
  (if (Variables|/Script/OneSoul.OnsSoulPlayer|Getkilltitan _asbp_player)
    (Utilities|FlowControl|DoOnce false
      (:Completed
        (Audio|Components|Audio|Stop (Variables|Default|GetNewVar_0))
        (bind _returnvalue (Audio|SpawnSound2D "/Game/LJW/mapContent/BackgroundMusic/Skyrim_Soundtrack__Silence_Unbroken.Skyrim_Soundtrack__Silence_Unbroken" 1.0 1.0 0.0 0))
        (Variables|Default|SetNewVar_0 _returnvalue)))))

(fn ConstructionScript)