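; BP_Enemy_Magician_magic2 is a short-lived fire spell effect actor for the magician enemy, with no damage or overlap logic of its own.
; BeginPlay plays a 2D fire sound, then after two seconds stops it and sets the Alpa flag.
; While flagged, Tick scales the particle system down multiplicatively each frame, so the shrink rate depends on frame rate.
; The actor destroys itself two seconds after shrinking begins.
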(event EventBeginPlay
  ;[1 1 1] 2초가지나면 점점 작아지고 다시 2초후 사라지는
  (bind _returnvalue (Audio|SpawnSound2D "/Game/LJW/Enemys/sound/Fire_by_SGAK_Id-87564.Fire_by_SGAK_Id-87564" 1.0 1.0 0.0 0))
  (Variables|Default|SetNewVar_0 _returnvalue)
  (Utilities|FlowControl|Delay 2.0)
  (Variables|Default|Setalpa true)
  (Audio|Components|Audio|Stop (Variables|Default|GetNewVar_0))
  (Utilities|FlowControl|Delay 2.0)
  (Actor|DestroyActor))

(event Collision|EventActorBeginOverlap
  (params (OtherActor :type Actor%20Object%20Reference)))

(event EventTick
  (params (DeltaSeconds :type Float%20%28single-precision%29))
  ;[1 1 1] 점점 작아지는
  (if (Variables|Default|Getalpa)
    (Transformation|SetWorldScale3D (Variables|Default|GetParticleSystem) (* (Transformation|GetWorldScale (Variables|Default|GetParticleSystem)) "0.900000,0.900000,0.900000"))))

(fn ConstructionScript)