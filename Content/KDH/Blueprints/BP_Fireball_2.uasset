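; BP_Fireball_2 is a fireball actor tied to BP_MountainDragon that travels downward and grows as it moves.
; On BeginPlay it caches the first dragon found in the level.
; Each tick it moves without sweep along the dragon capsule's negative up vector at a fixed speed and adds a constant, frame-rate-dependent scale increment.
; It destroys itself when the dragon reference becomes invalid, and has no hit or damage logic.
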(event EventBeginPlay
  (bind _returnvalue (Actor|GetActorOfClass "/Game/KDH/Blueprints/BP_MountainDragon.BP_MountainDragon_C"))
  (Variables|Default|Setme _returnvalue))

(event Collision|EventActorBeginOverlap
  (params (OtherActor :type Actor%20Object%20Reference)))

(event EventTick
  (params (DeltaSeconds :type Float%20%28single-precision%29))
  (Utilities|IsValid (Variables|Default|Getme)
    (:Is%20Valid
      (Transformation|SetActorLocation (+ (Transformation|GetActorLocation) (* (* (* (Math|Vector|GetUpVector (Variables|/Script/Engine.Character|GetCapsuleComponent (Variables|Default|Getme))) (Math|Float|MakeLiteralFloat -1.0)) (Math|Float|MakeLiteralFloat 1e+03)) DeltaSeconds)) false false)
      (Transformation|SetActorScale3D (+ (Transformation|GetActorScale3D) (Math|Float|MakeLiteralFloat 0.07))))
    (:Is%20Not%20Valid
      (Actor|DestroyActor))))

(fn ConstructionScript)